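; BP_RollerBall3DPlayer is the player Blueprint for the RollerBall3D game, handling HUD setup and a debug marker.
; On BeginPlay it creates the HUD widget, adds it to the viewport and passes it the first BP_RollerBall3DEnemy found, printing a warning if none is valid.
; Each Tick it draws a short-lived debug sphere at Destination, a value this graph reads but never sets.
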(event EventTick
  (params (DeltaSeconds :type Float%20%28single-precision%29))
  (Rendering|Debug|DrawDebugSphere (Variables|Default|GetDestination) 3e+01 24 "(R=1.000000,G=0.206515,B=0.000000,A=1.000000)" 0.05 1e+01))

(event EventBeginPlay
  (bind _returnvalue (UserInterface|CreateWidget "/Game/BP/RollerBall3D/WBP_RollerBall3DHUD.WBP_RollerBall3DHUD_C"))
  (bind _output_get (Variables|Default|SetHUD _returnvalue))
  (UserInterface|Viewport|AddtoViewport _output_get 0)
  (bind _outactors (Actor|GetAllActorsOfClass "/Game/BP/RollerBall3D/BP_RollerBall3DEnemy.BP_RollerBall3DEnemy_C"))
  (Utilities|IsValid (Utilities|Array|Get(acopy) _outactors)
    (:Is%20Valid
      (Variables|/Game/BP/RollerBall3D/WBP_RollerBall3DHUD.WBP_RollerBall3DHUD_C|SetEnemy (Variables|Default|GetHUD) (Utilities|Array|Get(acopy) _outactors)))
    (:Is%20Not%20Valid
      (Development|PrintString "No Enemy!"))))

(fn ConstructionScript)