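; BP_PlatformSwitcherPlayer is the player actor for the Platform Switcher game, handling HUD feedback, sound effects and respawn.
; On BeginPlay it creates and shows WBP_PlatformSwitcherHUD.
; Win and Lose events briefly display a result message on the HUD, and Lose also teleports the player back to StartLocation.
; Separate events play 2D sounds for jumping and teleporting.
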(event EventBeginPlay
  ;[1 1 1] HUD
  (bind _returnvalue (UserInterface|CreateWidget "/Game/BP/PlatformSwitcher/WBP_PlatformSwitcherHUD.WBP_PlatformSwitcherHUD_C"))
  (bind _output_get (Variables|Default|SetHUD _returnvalue))
  (UserInterface|Viewport|AddtoViewport _output_get 0))

(event EventPlayTeleportFX
  ;[1 1 1] Play FX
  (Audio|PlaySound2D "/Engine/VREditor/Sounds/UI/Teleport_Committed.Teleport_Committed" 0.5))

(event EventPlayJumpFX
  ;[1 1 1] Play FX
  (Audio|PlaySound2D "/Engine/VREditor/Sounds/UI/Drop_Item_From_ContentBrowser.Drop_Item_From_ContentBrowser" 0.5))

(event EventWin
  (bind _hud (Variables|Default|GetHUD))
  (bind _hud_text (Variables|/Game/BP/PlatformSwitcher/WBP_PlatformSwitcherHUD.WBP_PlatformSwitcherHUD_C|GetHUD_Text _hud))
  (Widget|SetVisibility _hud_text "Visible")
  (Rendering|Components|TextRender|SetText _hud_text "You Win !")
  (Utilities|FlowControl|Delay 2.0)
  (Widget|SetVisibility _hud_text "Hidden"))

(event EventLose
  (bind _hud (Variables|Default|GetHUD))
  (bind _hud_text (Variables|/Game/BP/PlatformSwitcher/WBP_PlatformSwitcherHUD.WBP_PlatformSwitcherHUD_C|GetHUD_Text _hud))
  ;[0 0.05874 0.5] Restart the game
  (Transformation|SetActorLocation (Variables|Default|GetStartLocation) false true)
  (Widget|SetVisibility _hud_text "Visible")
  (Rendering|Components|TextRender|SetText _hud_text "You Lose !")
  (Utilities|FlowControl|Delay 2.0)
  (Widget|SetVisibility _hud_text "Hidden"))

(fn ConstructionScript)