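; BP_MoveToSpawner is a spawner actor that creates instances of a configurable class inside its Box component's bounds.
; BeginPlay starts an optionally looping timer that calls Spawn by name after a set delay.
; When ShouldSpawn is true, Spawn places the actor at a random point in the box, rolls each scale axis independently within a configurable range, and applies the chosen collision handling.
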(event Custom|Spawn
  (bind _box (Variables|Default|GetBox))
  (bind _minscale (Variables|Default|GetMinScale))
  (bind _maxscale (Variables|Default|GetMaxScale))
  (bind _returnvalue (Math|Random|RandomFloatinRange _minscale _maxscale))
  (bind (_origin _boxextent) (Collision|GetComponentBounds _box))
  (if (Variables|Default|GetShouldSpawn)
    (Game|SpawnActorfromClass (Variables|Default|GetWhatToSpawn) (Math|Transform|MakeTransform (Math|Random|RandomPointinBoundingBox _origin _boxextent) "0, 0, 0" (Math|Vector|MakeVector _returnvalue _returnvalue _returnvalue)) (Variables|Default|GetCollisionHandling) 0 0)))

(event EventBeginPlay
  (Utilities|Time|SetTimerbyFunctionName 0 "Spawn" (Variables|Default|GetSpawningDelay) (Variables|Default|GetLooping)))

(fn ConstructionScript)