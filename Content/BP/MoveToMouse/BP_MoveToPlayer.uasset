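; BP_MoveToPlayer is the player actor for the MoveToMouse game, handling HUD, pickup feedback and end-of-game flow.
; BeginPlay adds the HUD widget to the viewport and scales the actor to half size.
; OnPickUp plays a success or failure sound based on its Correct flag.
; Win and lose events show an end-game widget with the result message, then share a short delay before reloading the current level.
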(event EventBeginPlay
  (bind _returnvalue (Math|Float|MakeLiteralFloat 0.5))
  ;[0 0.05874 0.5] HUD
  (bind _returnvalue_2 (UserInterface|CreateWidget "/Game/BP/MoveToMouse/WBP_MoveToHUDWidget.WBP_MoveToHUDWidget_C"))
  (UserInterface|Viewport|AddtoViewport _returnvalue_2 0)
  (Transformation|SetActorScale3D (Math|Vector|MakeVector _returnvalue _returnvalue _returnvalue)))

(event EventOnPickUp
  (params (bCorrect :type Boolean))
  (if bCorrect
    (Audio|PlaySound2D "/Engine/EditorSounds/Notifications/CompileSuccess_Cue.CompileSuccess_Cue")
    (else
      (Audio|PlaySound2D "/Engine/EditorSounds/Notifications/CompileFailed_Cue.CompileFailed_Cue"))))

(event EventWintheGame
  (bind _returnvalue (UserInterface|CreateWidget "/Game/BP/MoveToMouse/WBP_EndGameWidget.WBP_EndGameWidget_C" 0 "You Won the game !!!"))
  (UserInterface|Viewport|AddtoViewport _returnvalue 0)
  (Utilities|FlowControl|Delay 3.0)
  (bind _returnvalue_2 (Game|GetCurrentLevelName true))
  (Game|OpenLevel(byName) (Utilities|String|StringToName _returnvalue_2)))

(event EventLosetheGame
  (bind _returnvalue (UserInterface|CreateWidget "/Game/BP/MoveToMouse/WBP_EndGameWidget.WBP_EndGameWidget_C" 0 "You Lose the Game !!!"))
  (UserInterface|Viewport|AddtoViewport (stale EventWintheGame _returnvalue) 0)
  (Utilities|FlowControl|Delay 3.0)
  (bind _returnvalue_2 (Game|GetCurrentLevelName true))
  (Game|OpenLevel(byName) (Utilities|String|StringToName _returnvalue_2)))

(fn ConstructionScript)