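; Player Blueprint for a gravity platformer that owns the HUD and handles the win and lose end states.
; BeginPlay creates the HUD widget and adds it to the viewport.
; The win and lose events each pause the level timer, show their result message on the HUD and disable player input.
; Both then share a short delay that ends by reloading the current level.
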(event EventBeginPlay
  (bind _returnvalue (UserInterface|CreateWidget "/Game/BP/GravityPlatformer/WBP_GravityPlatformerHUD.WBP_GravityPlatformerHUD_C"))
  (bind _output_get (Variables|Default|SetHUD _returnvalue))
  (UserInterface|Viewport|AddtoViewport _output_get 0))

(event EventLosetheGame
  (bind _hud (Variables|Default|GetHUD))
  (bind _message (Variables|/Game/BP/GravityPlatformer/WBP_GravityPlatformerHUD.WBP_GravityPlatformerHUD_C|GetMessage _hud))
  (Utilities|Time|PauseTimerbyHandle (Variables|Default|GetLevelTimer))
  (Rendering|Components|TextRender|SetText _message "You Lose !")
  (Widget|SetVisibility _message "Visible")
  (Input|DisableInput (.AsPlayer%20Controller (Utilities|Casting|CastToPlayerController (Pawn|GetController))))
  (Utilities|FlowControl|Delay 3.0)
  (bind _returnvalue (Game|GetCurrentLevelName true))
  (Game|OpenLevel(byName) (Utilities|String|StringToName _returnvalue)))

(event EventWintheGame
  (bind _hud (Variables|Default|GetHUD))
  (bind _message (Variables|/Game/BP/GravityPlatformer/WBP_GravityPlatformerHUD.WBP_GravityPlatformerHUD_C|GetMessage _hud))
  (Utilities|Time|PauseTimerbyHandle (Variables|Default|GetLevelTimer))
  (Rendering|Components|TextRender|SetText _message "You Win !")
  (Widget|SetVisibility _message "Visible")
  (Input|DisableInput (.AsPlayer%20Controller (Utilities|Casting|CastToPlayerController (Pawn|GetController))))
  (Utilities|FlowControl|Delay 3.0)
  (bind _returnvalue (Game|GetCurrentLevelName true))
  (Game|OpenLevel(byName) (Utilities|String|StringToName _returnvalue)))

(fn ConstructionScript)